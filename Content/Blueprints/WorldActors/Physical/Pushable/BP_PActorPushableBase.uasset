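; Pushable world actor base that gets kicked a set distance along its local X or Y axis when its trigger boxes are overlapped.
; Each axis has a limited number of moves; a hit disables that box's collision and picks the sign of the kick distance.
; A local offset finds the end point, then a per-axis timeline lerps the actor there and re-enables the boxes' query collision.
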(event OnComponentBeginOverlap(Box-X)
  (params (OverlappedComponent :type Primitive%20Component%20Object%20Reference) (OtherActor :type Actor%20Object%20Reference) (OtherComp :type Primitive%20Component%20Object%20Reference) (OtherBodyIndex :type Integer) (bFromSweep :type Boolean) (SweepResult :type Hit%20Result%20Structure%20%28by%20ref%29))
  (bind __x_allowed (Variables|Default|Get-X%20allowed))
  ;[1 1 1] Handling of kicking
  (Math|Integer|CompareInt __x_allowed
    (:>
      (Math|Integer|DecrementInt __x_allowed
        (:%20%20
          (Collision|SetCollisionEnabled OverlappedComponent "NoCollision")
          (Math|Float|CompareFloat (Variables|Default|GetDistanceToKick) 0.0
            (:>
              (Variables|Default|SetDistanceToKick (* (Variables|Default|GetDistanceToKick) -1.0)))
            (:<
              _))
          (Variables|Default|SetStartLocation (Transformation|GetActorLocation))
          (Transformation|AddActorLocalOffset (Math|Vector|MakeVector (Variables|Default|GetDistanceToKick) 0.0 0.0) false false)
          (Variables|Default|SetEndLocation (Transformation|GetActorLocation))
          (bind _newtrack_0 (Timeline|Timeline_1 PlayFromStart)
            (:Update
              (Transformation|SetActorLocation (Math|Vector|Lerp(Vector) (Variables|Default|GetStartLocation) (Variables|Default|GetEndLocation) _newtrack_0) false false))
            (:Finished
              (Collision|SetCollisionEnabled (Variables|Default|GetBox-X) "QueryOnly"))))))))

(event OnComponentBeginOverlap(Box+X)
  (params (OverlappedComponent :type Primitive%20Component%20Object%20Reference) (OtherActor :type Actor%20Object%20Reference) (OtherComp :type Primitive%20Component%20Object%20Reference) (OtherBodyIndex :type Integer) (bFromSweep :type Boolean) (SweepResult :type Hit%20Result%20Structure%20%28by%20ref%29))
  (bind __x_allowed (Variables|Default|Get+X%20allowed))
  ;[1 1 1] Handling of kicking
  (Math|Integer|CompareInt __x_allowed
    (:>
      (Math|Integer|DecrementInt __x_allowed
        (:%20%20
          (Collision|SetCollisionEnabled OverlappedComponent "NoCollision")
          (Math|Float|CompareFloat (Variables|Default|GetDistanceToKick) 0.0
            (:>
              _)
            (:<
              (Variables|Default|SetDistanceToKick (* (Variables|Default|GetDistanceToKick) -1.0))))
          (Variables|Default|SetStartLocation (Transformation|GetActorLocation))
          (Transformation|AddActorLocalOffset (Math|Vector|MakeVector (Variables|Default|GetDistanceToKick) 0.0 0.0) false false)
          (Variables|Default|SetEndLocation (Transformation|GetActorLocation))
          (bind _newtrack_0 (Timeline|Timeline_1 PlayFromStart)
            (:Update
              (Transformation|SetActorLocation (Math|Vector|Lerp(Vector) (Variables|Default|GetStartLocation) (Variables|Default|GetEndLocation) _newtrack_0) false false))
            (:Finished
              (Collision|SetCollisionEnabled (Variables|Default|GetBox-X) "QueryOnly"))))))))

(event OnComponentBeginOverlap(Box-Y)
  (params (OverlappedComponent :type Primitive%20Component%20Object%20Reference) (OtherActor :type Actor%20Object%20Reference) (OtherComp :type Primitive%20Component%20Object%20Reference) (OtherBodyIndex :type Integer) (bFromSweep :type Boolean) (SweepResult :type Hit%20Result%20Structure%20%28by%20ref%29))
  (bind __y_allowed (Variables|Default|Get-Y%20allowed))
  ;[1 1 1] Handling of kicking
  (Math|Integer|CompareInt __y_allowed
    (:>
      (Math|Integer|DecrementInt __y_allowed
        (:%20%20
          (Collision|SetCollisionEnabled OverlappedComponent "NoCollision")
          (Math|Float|CompareFloat (Variables|Default|GetDistanceToKick) 0.0
            (:>
              (Variables|Default|SetDistanceToKick (* (Variables|Default|GetDistanceToKick) -1.0)))
            (:<
              _))
          (Variables|Default|SetStartLocation (Transformation|GetActorLocation))
          (Transformation|AddActorLocalOffset (Math|Vector|MakeVector 0.0 (Variables|Default|GetDistanceToKick) 0.0) false false)
          (Variables|Default|SetEndLocation (Transformation|GetActorLocation))
          (bind _newtrack_0 (Timeline|Timeline_2 PlayFromStart)
            (:Update
              (Transformation|SetActorLocation (Math|Vector|Lerp(Vector) (Variables|Default|GetStartLocation) (Variables|Default|GetEndLocation) _newtrack_0) false false))
            (:Finished
              (Collision|SetCollisionEnabled (Variables|Default|GetBox-Y) "QueryOnly"))))))))

(event OnComponentBeginOverlap(Box+Y)
  (params (OverlappedComponent :type Primitive%20Component%20Object%20Reference) (OtherActor :type Actor%20Object%20Reference) (OtherComp :type Primitive%20Component%20Object%20Reference) (OtherBodyIndex :type Integer) (bFromSweep :type Boolean) (SweepResult :type Hit%20Result%20Structure%20%28by%20ref%29))
  (bind __y_allowed (Variables|Default|Get+Y%20allowed))
  ;[1 1 1] Handling of kicking
  (Math|Integer|CompareInt __y_allowed
    (:>
      (Math|Integer|DecrementInt __y_allowed
        (:%20%20
          (Collision|SetCollisionEnabled OverlappedComponent "NoCollision")
          (Math|Float|CompareFloat (Variables|Default|GetDistanceToKick) 0.0
            (:>
              _)
            (:<
              (Variables|Default|SetDistanceToKick (* 0.0 -1.0))))
          (Variables|Default|SetStartLocation (Transformation|GetActorLocation))
          (Transformation|AddActorLocalOffset (Math|Vector|MakeVector 0.0 (Variables|Default|GetDistanceToKick) 0.0) false false)
          (Variables|Default|SetEndLocation (Transformation|GetActorLocation))
          (bind _newtrack_0 (Timeline|Timeline_2 PlayFromStart)
            (:Update
              (Transformation|SetActorLocation (Math|Vector|Lerp(Vector) (Variables|Default|GetStartLocation) (Variables|Default|GetEndLocation) _newtrack_0) false false))
            (:Finished
              (Collision|SetCollisionEnabled (Variables|Default|GetBox-Y) "QueryOnly"))))))))

(event EventBeginPlay
  (|CallParentFunction) ; This node is disabled and will not be called.\nDrag off pins to build functionality.
)

(event Collision|EventActorBeginOverlap
  (params (OtherActor :type Actor%20Object%20Reference))
  (|CallParentFunction OtherActor) ; This node is disabled and will not be called.\nDrag off pins to build functionality.
)

(event EventTick
  (params (DeltaSeconds :type Float%20%28single-precision%29))
  (|CallParentFunction DeltaSeconds) ; This node is disabled and will not be called.\nDrag off pins to build functionality.
)

(fn ConstructionScript
  (|CallParentFunction))