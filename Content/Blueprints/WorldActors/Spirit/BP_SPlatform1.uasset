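; Spirit world platform that carries the player between its placed position and a marker height, turning toward a fixed -90 yaw at the top.
; Each box overlap, unfiltered by actor, alternates between rising and descending, with timelines lerping location and rotation.
; During travel, the player pawn's input and tick are disabled and it is snap-attached to the platform.
; On arrival, both are restored, but the pawn is attached again rather than detached.
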(event OnComponentBeginOverlap(BoxCollision)
  (params (OverlappedComponent :type Primitive%20Component%20Object%20Reference) (OtherActor :type Actor%20Object%20Reference) (OtherComp :type Primitive%20Component%20Object%20Reference) (OtherBodyIndex :type Integer) (bFromSweep :type Boolean) (SweepResult :type Hit%20Result%20Structure%20%28by%20ref%29))
  (Utilities|FlowControl|FlipFlop
    (:A
      (CallFunction|TurnCharacterInputOff)
      (CallFunction|GoUp))
    (:B
      (CallFunction|TurnCharacterInputOff)
      (CallFunction|GoDown))))

(event Custom|GoUp
  (bind _newtrack_0 (Timeline|SmoothMotion PlayFromStart)
    (:Update
      (Transformation|SetActorTransform (Math|Transform|MakeTransform (Math|Vector|Lerp(Vector) (Variables|Default|GetGroundPosition) (Variables|Default|GetTopPosition) _newtrack_0) (Math|Rotator|Lerp(Rotator) (Variables|Default|GetGroundRotation) (Variables|Default|GetTopRotation) _newtrack_0) (Transformation|GetActorScale3D))))
    (:Finished
      (CallFunction|TurnCharacterInputon))))

(event Custom|GoDown
  (bind _newtrack_0 (Timeline|Timeline_0 PlayFromStart)
    (:Update
      (Transformation|SetActorTransform (Math|Transform|MakeTransform (Math|Vector|Lerp(Vector) (Variables|Default|GetTopPosition) (Variables|Default|GetGroundPosition) _newtrack_0) (Math|Rotator|Lerp(Rotator) (Variables|Default|GetTopRotation) (Variables|Default|GetGroundRotation) _newtrack_0) (Transformation|GetActorScale3D))))
    (:Finished
      (CallFunction|TurnCharacterInputon))))

(event EventBeginPlay
  (Variables|Default|SetGroundPosition (Transformation|GetActorLocation))
  (Variables|Default|SetTopPosition (Transformation|GetWorldLocation (Variables|Default|GetTopPosition%20Height)))
  (Variables|Default|SetGroundRotation (Transformation|GetActorRotation))
  (Variables|Default|SetTopRotation (Math|Rotator|MakeRotator (.roll (Variables|Default|GetGroundRotation)) (.pitch (Variables|Default|GetGroundRotation)) -9e+01)))

(event Collision|EventActorBeginOverlap
  (params (OtherActor :type Actor%20Object%20Reference)))

(event EventTick
  (params (DeltaSeconds :type Float%20%28single-precision%29)))

(fn ConstructionScript)

(fn TurnCharacterInputOff
  (bind _returnvalue (Game|GetPlayerController 0))
  (bind _returnvalue_2 (Pawn|GetControlledPawn _returnvalue))
  (Input|DisableInput _returnvalue_2 0)
  (Actor|Tick|SetActorTickEnabled _returnvalue_2)
  (Transformation|AttachActorToActor _returnvalue_2 self "None" "SnapToTarget" "KeepWorld" "KeepWorld" false))

(fn TurnCharacterInputon
  (bind _returnvalue (Game|GetPlayerController 0))
  (bind _returnvalue_2 (Pawn|GetControlledPawn _returnvalue))
  (Input|EnableInput _returnvalue_2 0)
  (Actor|Tick|SetActorTickEnabled _returnvalue_2 true)
  (Transformation|AttachActorToActor _returnvalue_2 self "None" "SnapToTarget" "KeepWorld" "KeepWorld" false))