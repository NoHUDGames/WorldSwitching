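; Spirit shield pickup actor for the world-switching game, extending a parent class that receives its mesh and sphere collider references on BeginPlay.
; Pickup feedback runs a guarded timeline that scales the actor up and lifts the mesh, then destroys it.
; A sensing timeline drives the shield light-up while the actor's world matches the game mode's, resetting on a mismatch or on completion, when it also hides the actor.
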(event EventBeginPlay
  (Class|SPickupShield|SetShieldMeshReference (Variables|Default|GetStaticMesh))
  (Class|SPickupShield|SetSphereColliderReference (Variables|Default|GetSphere))
  (bind _asbp_world_switching_game_mode (Utilities|Casting|CastToBP_WorldSwitchingGameMode (Game|GetGameMode)))
  (Variables|Default|SetGameModeRef _asbp_world_switching_game_mode))

(event Collision|EventActorBeginOverlap
  (params (OtherActor :type Actor%20Object%20Reference)))

(event EventTick
  (params (DeltaSeconds :type Float%20%28single-precision%29)))

(event EventPickupFeedback
  (if (not (Variables|Default|GetEffectIsRunning))
    (Variables|Default|SetEffectIsRunning true)
    (bind _floatup (Timeline|Timeline_0 PlayFromStart)
      (:Update
        (Transformation|SetActorScale3D (Math|Vector|MakeVector (Math|Float|Lerp 1.0 3.0 _floatup) (Math|Float|Lerp 1.0 3.0 _floatup) (Math|Float|Lerp 1.0 3.0 _floatup)))
        (Transformation|AddLocalOffset (Variables|Default|GetStaticMesh) (Math|Vector|MakeVector 0.0 0.0 (Math|Float|Lerp 0.0 1.0 _floatup)) false false))
      (:Finished
        (Actor|DestroyActor)
        (Variables|Default|SetEffectIsRunning false)))))

(event EventTriggerShieldLightUpTimeline
  (bind _newtrack_0 (Timeline|ShieldSensing PlayFromStart)
    (:Update
      (if (Math|Boolean|Equal(Boolean) (Variables|Default|Getm_bIsSpiritWorld) (Variables|/Script/WorldSwitching.WorldSwitchingGameModeBase|GetbIsSpiritWorld (Variables|Default|GetGameModeRef)))
        (Class|SPickupShield|LightUpShield _newtrack_0)
        (else
          (Class|SPickupShield|ResetAfterLightUp)
          (Timeline|ShieldSensing Stop))))
    (:Finished
      (Class|SPickupShield|ResetAfterLightUp)
      (Rendering|SetActorHiddenInGame true))))

(fn ConstructionScript)