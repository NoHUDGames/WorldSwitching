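; Spirit fire puzzle actor that opens sliding doors once both of its fires are lit.
; Left and right colliders respond only to BP_SFireStarter overlaps, each activating its fire component and setting a lit flag.
; When both flags are true, it finds every BP_PSSlidingDoor1 in the level by class and calls OpenDoor on each, rather than targeting a specific linked door.
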(event OnComponentBeginOverlap(LeftCollider)
  (params (OverlappedComponent :type Primitive%20Component%20Object%20Reference) (OtherActor :type Actor%20Object%20Reference) (OtherComp :type Primitive%20Component%20Object%20Reference) (OtherBodyIndex :type Integer) (bFromSweep :type Boolean) (SweepResult :type Hit%20Result%20Structure%20%28by%20ref%29))
  (Utilities|Casting|CastToBP_SFireStarter OtherActor)
  (Components|Activation|Activate (Variables|Default|GetFireLeft) false)
  (Variables|Default|SetbIsLeftLit true)
  (if (Variables|Default|GetbIsLeftLit)
    (if (Variables|Default|GetbIsRightLit)
      (bind _outactors (Actor|GetAllActorsOfClass "/Game/Blueprints/WorldActors/Both/BP_PSSlidingDoor1.BP_PSSlidingDoor1_C"))
      (bind _output_get (Variables|Default|SetSlidingDoorRef _outactors))
      (for _array_element _output_get
        (Default|OpenDoor _array_element)))))

(event OnComponentBeginOverlap(RightCollider)
  (params (OverlappedComponent :type Primitive%20Component%20Object%20Reference) (OtherActor :type Actor%20Object%20Reference) (OtherComp :type Primitive%20Component%20Object%20Reference) (OtherBodyIndex :type Integer) (bFromSweep :type Boolean) (SweepResult :type Hit%20Result%20Structure%20%28by%20ref%29))
  (Utilities|Casting|CastToBP_SFireStarter OtherActor)
  (Components|Activation|Activate (Variables|Default|GetFireRight) false)
  (Variables|Default|SetbIsRightLit true)
  (if (Variables|Default|GetbIsLeftLit)
    (if (Variables|Default|GetbIsRightLit)
      (bind _outactors (Actor|GetAllActorsOfClass "/Game/Blueprints/WorldActors/Both/BP_PSSlidingDoor1.BP_PSSlidingDoor1_C"))
      (bind _output_get (Variables|Default|SetSlidingDoorRef _outactors))
      (for _array_element _output_get
        (Default|OpenDoor _array_element)))))

(event EventBeginPlay)

(event Collision|EventActorBeginOverlap
  (params (OtherActor :type Actor%20Object%20Reference)))

(event EventTick
  (params (DeltaSeconds :type Float%20%28single-precision%29)))

(fn ConstructionScript)