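; BP_SCube is a spirit-world cube actor that lights up when sensed.
; On BeginPlay it registers its static mesh and caches the world-switching game mode.
; The light-up trigger records the current world and plays a timeline that drives TimeLineLightUp, restoring original materials when finished or stopping early if the world switches.
; Its logic duplicates SWorldActorBase because the asset was copied rather than derived from it.
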(event EventBeginPlay
  (Class|SWorldActor|SetMeshRef (Variables|Default|GetStaticMesh))
  (bind _asbp_world_switching_game_mode (Utilities|Casting|CastToBP_WorldSwitchingGameMode (Game|GetGameMode)))
  (Variables|Default|SetGameModeRef _asbp_world_switching_game_mode))

(event Collision|EventActorBeginOverlap
  (params (OtherActor :type Actor%20Object%20Reference)))

(event EventTick
  (params (DeltaSeconds :type Float%20%28single-precision%29)))

(event EventTimeLineLightUpTrigger
  (bind _gamemoderef (Variables|Default|GetGameModeRef))
  (bind _bisspiritworld (Variables|/Script/WorldSwitching.WorldSwitchingGameModeBase|GetbIsSpiritWorld _gamemoderef))
  ;[1 1 1] Light up when sensed. Was duplicate of SWorldActorBase, not derived from, hence duplicate code
  (Variables|Default|SetbIsSpiritWorldWhenTriggered _bisspiritworld)
  (bind _lightup (Timeline|Timeline_0 PlayFromStart)
    (:Update
      (if (Math|Boolean|Equal(Boolean) (Variables|Default|GetbIsSpiritWorldWhenTriggered) _bisspiritworld)
        (Class|SWorldActor|TimeLineLightUp _lightup)
        (else
          (Class|SWorldActor|ReapplyOriginalMaterials)
          (Timeline|Timeline_0 Stop))))
    (:Finished
      (Class|SWorldActor|ReapplyOriginalMaterials))))

(fn ConstructionScript)