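; Wall torch actor that toggles between lit and unlit whenever something begins overlapping its capsule.
; BeginPlay creates a dynamic material on the candle mesh and applies the StartLit state, though that lit branch leaves the parameter name as None instead of Glow.
; Each toggle sets IsLit, the Glow scalar and the DynamicBothWorlds component's activation.
; Extinguishing also calls GetAllActorsWithInterface, but the result is unused.
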(event OnComponentBeginOverlap(Capsule)
  (params (OverlappedComponent :type Primitive%20Component%20Object%20Reference) (OtherActor :type Actor%20Object%20Reference) (OtherComp :type Primitive%20Component%20Object%20Reference) (OtherBodyIndex :type Integer) (bFromSweep :type Boolean) (SweepResult :type Hit%20Result%20Structure%20%28by%20ref%29))
  (bind _torchmid (Variables|DynamicMaterial|GetTorchMID))
  (bind _dynamicbothworlds (Variables|Default|GetDynamicBothWorlds))
  (if (Variables|Default|GetbIsLit)
    (Rendering|Material|SetScalarParameterValue _torchmid "Glow" 1.0 :!class /Script/Engine.MaterialInstanceDynamic)
    (Components|Activation|Deactivate _dynamicbothworlds)
    (Variables|Default|SetbIsLit false)
    (Actor|GetAllActorswithInterface 0)
    (else
      (Rendering|Material|SetScalarParameterValue _torchmid "Glow" 1e+01 :!class /Script/Engine.MaterialInstanceDynamic)
      (Components|Activation|Activate _dynamicbothworlds false)
      (Variables|Default|SetbIsLit true))))

(event EventBeginPlay
  (bind _returnvalue (Rendering|Material|CreateDynamicMaterialInstance (Variables|Default|Getcandle) 0 0 "None" :!class /Script/Engine.PrimitiveComponent))
  (Variables|DynamicMaterial|SetTorchMID _returnvalue)
  (if (Variables|BeginPlay|GetbStartLit)
    (Components|Activation|Activate (Variables|Default|GetDynamicBothWorlds) false)
    (Rendering|Material|SetScalarParameterValue (Variables|DynamicMaterial|GetTorchMID) "None" 1e+01 :!class /Script/Engine.MaterialInstanceDynamic)
    (Variables|Default|SetbIsLit true)
    (else
      (Rendering|Material|SetScalarParameterValue (Variables|DynamicMaterial|GetTorchMID) "Glow" 1.0 :!class /Script/Engine.MaterialInstanceDynamic))))

(event Collision|EventActorBeginOverlap
  (params (OtherActor :type Actor%20Object%20Reference)))

(event EventTick
  (params (DeltaSeconds :type Float%20%28single-precision%29)))

(fn ConstructionScript)