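; Player character Blueprint that turns to face the mouse cursor and manages the HUD and pause menu.
; Each Tick it deprojects the cursor, traces against WorldStatic objects and sets its yaw toward the impact point.
; BeginPlay shows the cursor and adds the temporary health and artifact display outside the MainMenu level.
; Pause reuses one PauseMenu widget with UI-only input, while Unpause removes all widgets and restores game-only input.
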(event EventBeginPlay
  (Variables|/Script/Engine.PlayerController|SetbShowMouseCursor (Game|GetPlayerController 0) true)
  (bind _returnvalue (Game|GetCurrentLevelName true))
  (if (not (Utilities|Enum|Equal(Enum) _returnvalue "MainMenu"))
    (bind _returnvalue_2 (UserInterface|CreateWidget "/Game/HUD/TempHealthAndArtifactDisplay.TempHealthAndArtifactDisplay_C"))
    (UserInterface|Viewport|AddtoViewport _returnvalue_2 0)))

(event Collision|EventActorBeginOverlap
  (params (OtherActor :type Actor%20Object%20Reference)))

(event EventTick
  (params (DeltaSeconds :type Float%20%28single-precision%29))
  (bind _returnvalue (Game|GetPlayerController 0))
  (bind (_worldlocation _worlddirection) (Game|Player|ConvertMouseLocationToWorldSpace _returnvalue))
  (bind _outhit (Collision|LineTraceForObjects _worldlocation (+ _worldlocation (* _worlddirection 10000)) (Utilities|Array|MakeArray "ObjectTypeQuery1") false 0 "None"))
  (Transformation|SetActorRotation (Math|Rotator|MakeRotator 0.0 0.0 (.yaw (Math|Rotator|FindLookatRotation (Transformation|GetActorLocation) (.ImpactPoint (Collision|BreakHitResult _outhit)))))))

(event Input|ActionEvents|InputActionPauseMenu
  (params (Key :type Key%20Structure))
  ;[1 1 1] Pause the game
  (:Pressed
    (CallFunction|Pause)))

(fn ConstructionScript)

(fn Pause
  (bind _returnvalue (Game|GetPlayerController 0))
  (Game|SetGamePaused true)
  (Utilities|IsValid 0
    (:Is%20Valid
      _)
    (:Is%20Not%20Valid
      (bind _returnvalue_2 (UserInterface|CreateWidget "/Game/HUD/PauseMenu.PauseMenu_C" (Game|GetPlayerController 0)))
      (bind _output_get (Variables|Default|SetPauseMenu _returnvalue_2))))
  (UserInterface|Viewport|AddtoViewport _output_get 0)
  (Input|SetInputModeUIOnly _returnvalue (Variables|Default|GetPauseMenu) "DoNotLock")
  (Variables|/Script/Engine.PlayerController|SetbShowMouseCursor _returnvalue true))

(fn Unpause
  (Game|SetGamePaused false)
  (Viewport|RemoveAllWidgets)
  (Input|SetInputModeGameOnly (Game|GetPlayerController 0)))