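; Player character Blueprint that turns to face the mouse cursor or a locked-on enemy.
; The targeting input traces under the cursor to set or clear the lock on a Character.
; Tick handles rotation and the targeting beam, whose end point a timeline lerps from its spawn point to the enemy.
; It also shows the cursor, adds a temporary health and artifact display outside MainMenu, and manages the pause menu.
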(event EventBeginPlay
  (Variables|/Script/Engine.PlayerController|SetbShowMouseCursor (Game|GetPlayerController 0) true)
  (bind _returnvalue (Game|GetCurrentLevelName true))
  (if (not (Utilities|Enum|Equal(Enum) _returnvalue "MainMenu"))
    (bind _returnvalue_2 (UserInterface|CreateWidget "/Game/HUD/TempHealthAndArtifactDisplay.TempHealthAndArtifactDisplay_C"))
    (UserInterface|Viewport|AddtoViewport _returnvalue_2 0)))

(event Collision|EventActorBeginOverlap
  (params (OtherActor :type Actor%20Object%20Reference)))

(event EventTick
  (params (DeltaSeconds :type Float%20%28single-precision%29))
  (bind _returnvalue (Game|GetPlayerController 0))
  (bind _targetbeamspawnlocation (Variables|Default|GetTargetBeamSpawnLocation))
  (bind (_worldlocation _worlddirection) (Game|Player|ConvertMouseLocationToWorldSpace _returnvalue))
  (bind _returnvalue_2 (Transformation|GetWorldLocation _targetbeamspawnlocation))
  (Variables|Default|SetDeltaSeconds DeltaSeconds)
  (if (!= (Variables|Default|GetEnemyTarget) 0)
    (if (and (Variables|Default|GetisTargetingEnemy) (Utilities|IsValid (Variables|Default|GetEnemyTarget)))
      (Transformation|SetActorRotation (Math|Rotator|MakeRotator 0.0 0.0 (.yaw (Math|Rotator|FindLookatRotation (Transformation|GetActorLocation) (Transformation|GetActorLocation (Variables|Default|GetEnemyTarget))))))
      (if (Variables|Default|GetTargetBeamCurrentlyActive)
        (bind _newtrack_0 (Timeline|TargetingBeamTimeline Play)
          (:Update
            (if (and (Utilities|IsValid (Variables|Default|GetTargetBeam)) (Utilities|IsValid (Variables|Default|GetEnemyTarget)))
              (Class|ParticleSystemComponent|SetBeamSourcePoint (Variables|Default|GetTargetBeam) 0 _returnvalue_2)
              (Class|ParticleSystemComponent|SetBeamTargetPoint (Variables|Default|GetTargetBeam) 0 (Math|Vector|Lerp(Vector) _returnvalue_2 (Transformation|GetActorLocation (Variables|Default|GetEnemyTarget)) _newtrack_0))
              (Variables|Default|SetTargetBeamCurrentlyActive true))))
        (else
          (bind _returnvalue_3 (Effects|SpawnEmitteratLocation "/Game/ParticleEffects/TargetBeam/TargetBeam.TargetBeam" (Transformation|GetActorLocation)))
          (Variables|Default|SetTargetBeam _returnvalue_3)
          (Timeline|TargetingBeamTimeline PlayFromStart)))
      (else
        (bind _outhit (Collision|LineTraceForObjects _worldlocation (+ _worldlocation (* _worlddirection 10000)) (Utilities|Array|MakeArray "ObjectTypeQuery12") false 0 "None" :!label _label))
        (Transformation|SetActorRotation (Math|Rotator|MakeRotator 0.0 0.0 (.yaw (Math|Rotator|FindLookatRotation (Transformation|GetActorLocation) (.ImpactPoint (Collision|BreakHitResult _outhit))))))
        (if (Utilities|IsValid (Variables|Default|GetTargetBeam))
          (if (Components|Activation|IsActive (Variables|Default|GetTargetBeam))
            (Components|Activation|Deactivate (Variables|Default|GetTargetBeam))
            (Variables|Default|SetTargetBeamCurrentlyActive false)))))
    (else
      (goto _label))))

(event Input|ActionEvents|InputActionPauseMenu
  (params (Key :type Key%20Structure))
  ;[1 1 1] Pause the game
  (:Pressed
    (CallFunction|Pause)))

(event Input|ActionEvents|InputActionTargetingEnemy
  (params (Key :type Key%20Structure))
  (bind _returnvalue (Game|GetPlayerController 0))
  (bind (_worldlocation _worlddirection) (Game|Player|ConvertMouseLocationToWorldSpace _returnvalue))
  (:Pressed
    (bind _outactors (Actor|GetAllActorsOfClass "BP_Character_BP_C"))
    (bind _outhit (Collision|LineTraceForObjects _worldlocation (+ _worldlocation (* _worlddirection 10000)) (Utilities|Array|MakeArray "ObjectTypeQuery7" "ObjectTypeQuery8") false _outactors "None"))
    (Utilities|Casting|CastToCharacter (.HitActor (Collision|BreakHitResult _outhit))
      (:then
        (Variables|Default|SetEnemyTarget (.HitActor (Collision|BreakHitResult _outhit)))
        (Variables|Default|SetisTargetingEnemy true))
      (:CastFailed
        (Variables|Default|SetisTargetingEnemy false)))))

(fn ConstructionScript)

(fn Pause
  (bind _returnvalue (Game|GetPlayerController 0))
  (Game|SetGamePaused true)
  (Utilities|IsValid 0
    (:Is%20Valid
      _)
    (:Is%20Not%20Valid
      (bind _returnvalue_2 (UserInterface|CreateWidget "/Game/HUD/PauseMenu.PauseMenu_C" (Game|GetPlayerController 0)))
      (bind _output_get (Variables|Default|SetPauseMenu _returnvalue_2))))
  (UserInterface|Viewport|AddtoViewport _output_get 0)
  (Input|SetInputModeUIOnly _returnvalue (Variables|Default|GetPauseMenu) "DoNotLock")
  (Variables|/Script/Engine.PlayerController|SetbShowMouseCursor _returnvalue true))

(fn Unpause
  (Game|SetGamePaused false)
  (Viewport|RemoveAllWidgets)
  (Input|SetInputModeGameOnly (Game|GetPlayerController 0)))

(fn TargetingBeam)