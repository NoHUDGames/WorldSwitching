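; Game mode for a world-switching game, providing the feedback effects for changing worlds and for denied re-entry to the physical world.
; Transitions play a sound with a timeline-driven pulse of camera post-process settings, while denial triggers a camera shake.
; LightUpCollidingActor briefly reveals an S- or P-world actor by swapping in a glowing dynamic material and fading its opacity, then re-hides it and restores the material, guarded against overlapping runs.
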(event EventBeginPlay
  (Development|PrintString "GameModeBeginPlayRuns")
  (Variables|/Script/Engine.PlayerController|SetCurrentMouseCursor (Game|GetPlayerController 0) "CardinalCross"))

(event EventTick
  (params (DeltaSeconds :type Float%20%28single-precision%29)))

(event EventWorldTransitionEffects
  (Audio|PlaySound2D "/Game/Sound/ChangeWorld.ChangeWorld" 1.0 1.0 0.0 0 0)
  (bind _returnvalue (Class|WorldSwitchingGameModeBase|GetPawnCameraComponent))
  (bind (_direction _0_5_sec_010 _newtrack_0) (Timeline|Timeline_0 PlayFromStart)
    (:Update
      (Utilities|Struct|SetmembersinPostProcessSettings (Variables|/Script/Engine.CameraComponent|GetPostProcessSettings _returnvalue) "DOFM_BokehDOF" 0.0 (Math|Float|Lerp 0.0 2.0 _0_5_sec_010) (Math|Float|Lerp 0.0 2.0 _0_5_sec_010) (Math|Float|Lerp 0.0 1.5 _newtrack_0) (Math|Float|Lerp 0.0 2.0 _0_5_sec_010) (Math|Float|Lerp 0.0 2.0 _0_5_sec_010) (Math|Float|Lerp 0.0 2.0 _0_5_sec_010)))))

(event EventDeniedPhysicalReentryEffects
  (bind _returnvalue (Class|WorldSwitchingGameModeBase|GetPawnCameraComponent))
  (Camera|PlayWorldCameraShake "/Game/Blueprints/CameraShakes/DeniedShake.DeniedShake_C" (Transformation|GetWorldLocation _returnvalue) 3.0 4.0))

(event EventLightUpCollidingActor
  (params (SWordActor :type S%20World%20Actor%20Object%20Reference) (PWorldActor :type P%20World%20Actor%20Object%20Reference))
  (if (not (Variables|Default|GetbLightUpEffectsRunning))
    (Variables|Default|SetbLightUpEffectsRunning true)
    (if (Utilities|IsValid SWordActor)
      (Variables|Default|SetOtherActorRef SWordActor)
      (elif (Utilities|IsValid PWorldActor)
        (Variables|Default|SetOtherActorRef PWorldActor)
        (else
          (bind _returnvalue (Class|WorldSwitchingGameModeBase|GetOtherActorPhysicalTest))
          (Variables|Default|SetOtherActorRef _returnvalue))))
    (Variables|Default|SetMeshRef (Actor|GetComponentbyClass (Variables|Default|GetOtherActorRef) "/Script/Engine.StaticMeshComponent"))
    (Variables|Default|SetOriginalMaterialRef (Rendering|Material|GetMaterial (Actor|GetComponentbyClass (Variables|Default|GetOtherActorRef) "/Script/Engine.StaticMeshComponent") 0))
    (Utilities|Casting|CastToPWorldActor (Variables|Default|GetOtherActorRef)
      (:then
        (Rendering|Material|SetMaterial (Variables|Default|GetMeshRef) 0 "/Game/Materials/M_SensingDummyLight_P.M_SensingDummyLight_P"))
      (:CastFailed
        (Utilities|Casting|CastToSWorldActor (Variables|Default|GetOtherActorRef))
        (Rendering|Material|SetMaterial (Variables|Default|GetMeshRef) 0 0)))
    (bind _returnvalue_2 (Rendering|Material|CreateDynamicMaterialInstance (Variables|Default|GetMeshRef) 0 0 "None" :!class /Script/Engine.PrimitiveComponent))
    (bind _output_get (Variables|Default|SetMaterialInstanceDynamic _returnvalue_2))
    (bind _returnvalue_3 (Rendering|Material|GetVectorParameterValue _output_get "BaseColor" :!class /Script/Engine.MaterialInstanceDynamic))
    (Variables|Default|SetFOriginalColor _returnvalue_3)
    (Rendering|Material|SetScalarParameterValue (Variables|Default|GetMaterialInstanceDynamic) "Opacity" 0.0 :!class /Script/Engine.MaterialInstanceDynamic)
    (Rendering|Material|SetScalarParameterValue (Variables|Default|GetMaterialInstanceDynamic) "Glow" 5e+01 :!class /Script/Engine.MaterialInstanceDynamic)
    (Rendering|SetActorHiddenInGame (Variables|Default|GetOtherActorRef) false)
    (bind _fadeinout (Timeline|Timeline_1 PlayFromStart)
      (:Update
        (Rendering|Material|SetScalarParameterValue (Variables|Default|GetMaterialInstanceDynamic) "Opacity" _fadeinout :!class /Script/Engine.MaterialInstanceDynamic))
      (:Finished
        (Rendering|SetActorHiddenInGame (Variables|Default|GetOtherActorRef) true)
        (Rendering|Material|SetMaterial (Variables|Default|GetMeshRef) 0 (Variables|Default|GetOriginalMaterialRef))
        (Variables|Default|SetbLightUpEffectsRunning false)))))

(fn ConstructionScript)