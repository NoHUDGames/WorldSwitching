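; BP_Character is a character Blueprint that turns to face the point in the world under the mouse cursor.
; BeginPlay shows the cursor on the first player controller.
; Each Tick deprojects the cursor into a line trace against WorldStatic objects, then applies only the yaw of the look-at rotation toward the impact point.
; The trace result is used without checking for a hit.
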(event EventBeginPlay
  (Variables|/Script/Engine.PlayerController|SetbShowMouseCursor (Game|GetPlayerController 0) true))

(event Collision|EventActorBeginOverlap
  (params (OtherActor :type Actor%20Object%20Reference)))

(event EventTick
  (params (DeltaSeconds :type Float%20%28single-precision%29))
  (bind _returnvalue (Game|GetPlayerController 0))
  (bind (_worldlocation _worlddirection) (Game|Player|ConvertMouseLocationToWorldSpace _returnvalue))
  (bind _outhit (Collision|LineTraceForObjects _worldlocation (+ _worldlocation (* _worlddirection 10000)) (Utilities|Array|MakeArray "ObjectTypeQuery1") false 0 "None"))
  (Transformation|SetActorRotation (Math|Rotator|MakeRotator 0.0 0.0 (.yaw (Math|Rotator|FindLookatRotation (Transformation|GetActorLocation) (.ImpactPoint (Collision|BreakHitResult _outhit)))))))

(fn ConstructionScript)