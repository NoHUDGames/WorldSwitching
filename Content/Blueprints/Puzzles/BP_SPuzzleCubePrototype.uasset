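; Prototype puzzle cube Blueprint that handles a timed light-up effect and a player collision reset.
; On BeginPlay it registers its static mesh through SetMeshRef.
; TimeLineLightUpTrigger plays a timeline that feeds TimeLineLightUp each update, then calls ReapplyOriginalMaterials when finished.
; When any overlap with the mesh ends, player 0's capsule is set to block GameTraceChannel1.
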(event OnComponentEndOverlap(StaticMesh)
  (params (OverlappedComponent :type Primitive%20Component%20Object%20Reference) (OtherActor :type Actor%20Object%20Reference) (OtherComp :type Primitive%20Component%20Object%20Reference) (OtherBodyIndex :type Integer))
  (Collision|SetCollisionResponsetoChannel (Actor|GetComponentbyClass (Game|GetPlayerCharacter 0) "/Script/Engine.CapsuleComponent") "ECC_GameTraceChannel1" "ECR_Block"))

(event EventBeginPlay
  (Class|SWorldActor|SetMeshRef (Variables|Default|GetStaticMesh)))

(event Collision|EventActorBeginOverlap
  (params (OtherActor :type Actor%20Object%20Reference)))

(event EventTick
  (params (DeltaSeconds :type Float%20%28single-precision%29)))

(event EventTimeLineLightUpTrigger
  (Development|PrintString "TIMELINELIGHTUPTRIGGER CALLED")
  (bind _lightup (Timeline|Timeline_0 PlayFromStart)
    (:Update
      (Class|SWorldActor|TimeLineLightUp _lightup))
    (:Finished
      (Class|SWorldActor|ReapplyOriginalMaterials))))

(fn ConstructionScript)