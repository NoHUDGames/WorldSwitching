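; Tutorial sensing-puzzle bridge whose mesh is moved along local Y by a timeline and can light up when triggered.
; Tick flip-flops that timeline between play-from-start and reverse-from-end every frame.
; The light-up timeline restores original materials when it finishes or when the game mode's spirit-world state changes mid-effect.
; Ending overlap with the mesh sets the player capsule to block GameTraceChannel1.
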(event OnComponentEndOverlap(StaticMesh)
  (params (OverlappedComponent :type Primitive%20Component%20Object%20Reference) (OtherActor :type Actor%20Object%20Reference) (OtherComp :type Primitive%20Component%20Object%20Reference) (OtherBodyIndex :type Integer))
  (Collision|SetCollisionResponsetoChannel (Actor|GetComponentbyClass (Game|GetPlayerCharacter 0) "/Script/Engine.CapsuleComponent") "ECC_GameTraceChannel1" "ECR_Block"))

(event EventBeginPlay
  (Class|SWorldActor|SetMeshRef (Variables|Default|GetStaticMesh))
  (bind _asbp_world_switching_game_mode (Utilities|Casting|CastToBP_WorldSwitchingGameMode (Game|GetGameMode)))
  (Variables|Default|SetGameModeRef _asbp_world_switching_game_mode))

(event Collision|EventActorBeginOverlap
  (params (OtherActor :type Actor%20Object%20Reference)))

(event EventTick
  (params (DeltaSeconds :type Float%20%28single-precision%29))
  (Utilities|FlowControl|FlipFlop
    (:A
      (bind _newtrack_0 (Timeline|Timeline_1 PlayFromStart)
        (:Update
          (Transformation|SetRelativeLocation (Variables|Default|GetStaticMesh) (Math|Vector|MakeVector 245.0 _newtrack_0 -6.0) false false))))
    (:B
      (Timeline|Timeline_1 ReverseFromEnd))))

(event EventTimeLineLightUpTrigger
  (bind _gamemoderef (Variables|Default|GetGameModeRef))
  (bind _bisspiritworld (Variables|/Script/WorldSwitching.WorldSwitchingGameModeBase|GetbIsSpiritWorld _gamemoderef))
  (Variables|Default|SetbIsSpiritWorldWhenTriggered _bisspiritworld)
  (bind _lightup (Timeline|Timeline_0 PlayFromStart)
    (:Update
      (if (Math|Boolean|Equal(Boolean) _bisspiritworld (Variables|Default|GetbIsSpiritWorldWhenTriggered))
        (Class|SWorldActor|TimeLineLightUp _lightup)
        (else
          (Class|SWorldActor|ReapplyOriginalMaterials)
          (Timeline|Timeline_0 Stop))))
    (:Finished
      (Class|SWorldActor|ReapplyOriginalMaterials))))

(fn ConstructionScript)