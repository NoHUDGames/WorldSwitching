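; BP_TutLev_PBridge1 is a bridge piece for the tutorial sensing puzzle that moves its static mesh vertically.
; The Move timeline lerps the mesh's relative Z between a lower and an upper location.
; Tick drives a FlipFlop that alternates PlayFromStart and ReverseFromEnd on every tick, with no gate or completion check, so the timeline restarts from alternating ends each frame.
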(event EventBeginPlay
  (|CallParentFunction) ; This node is disabled and will not be called.\nDrag off pins to build functionality.
)

(event Collision|EventActorBeginOverlap
  (params (OtherActor :type Actor%20Object%20Reference))
  (|CallParentFunction OtherActor) ; This node is disabled and will not be called.\nDrag off pins to build functionality.
)

(event EventTick
  (params (DeltaSeconds :type Float%20%28single-precision%29))
  (|CallParentFunction DeltaSeconds)
  (Utilities|FlowControl|FlipFlop
    (:A
      (bind _newtrack_0 (Timeline|Move PlayFromStart)
        (:Update
          (Transformation|SetRelativeLocation (Variables|Default|GetStaticMesh) (Math|Vector|MakeVector 0.0 0.0 (Math|Float|Lerp (Variables|Default|GetLowerZLocaction) (Variables|Default|GetUpperZLocation) _newtrack_0)) false false))))
    (:B
      (Timeline|Move ReverseFromEnd))))

(fn ConstructionScript
  (|CallParentFunction))