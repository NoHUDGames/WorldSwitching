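; Battle puzzle actor that shuts the player in with a moving wall and plays a camera cutaway at the start and on completion.
; Overlapping the closing trigger disables player input and idles the character, while Tick polls PuzzleFinished, which is not set here.
; Both run a shared one-shot delayed sequence that blends to a repositioned level camera, activates the wall only if unfinished, then restores view and input.
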(event OnComponentBeginOverlap(ClosingTrigger)
  (params (OverlappedComponent :type Primitive%20Component%20Object%20Reference) (OtherActor :type Actor%20Object%20Reference) (OtherComp :type Primitive%20Component%20Object%20Reference) (OtherBodyIndex :type Integer) (bFromSweep :type Boolean) (SweepResult :type Hit%20Result%20Structure%20%28by%20ref%29))
  (bind _returnvalue (Game|GetPlayerController 0))
  (bind _characterref (Variables|Default|GetCharacterRef))
  (Collision|SetCollisionEnabled (Variables|Default|GetClosingTrigger) "NoCollision")
  (Input|DisableInput _characterref (Game|GetPlayerController 0))
  (Variables|/Script/WorldSwitching.BP_Character|SetRunningAnimations _characterref "IDLE")
  (Utilities|FlowControl|DoOnce false
    (:Completed
      (Utilities|FlowControl|Delay 1.0)
      (Transformation|SetActorLocationAndRotation (Variables|Default|GetFreeLevelCamera) (Transformation|GetWorldLocation (Variables|Default|GetCameraLocation)) (Math|Rotator|FindLookatRotation (Transformation|GetWorldLocation (Variables|Default|GetCameraLocation)) (Transformation|GetWorldLocation (Variables|Default|GetCameraLookat))))
      (Game|Player|SetViewTargetwithBlend (Game|GetPlayerController 0) (Variables|Default|GetFreeLevelCamera) 1.0 "VTBlend_Linear" 0.0 false)
      (Utilities|FlowControl|Delay 1.5)
      (if (Variables|Default|GetPuzzleFinished)
        _
        (else
          (Variables|/Script/WorldSwitching.PSMovingWall|SetActivateMoving (Variables|Default|GetMovingWallActor) true)))
      (Utilities|FlowControl|Delay 2.0)
      (Game|Player|SetViewTargetwithBlend _returnvalue (Pawn|GetControlledPawn _returnvalue) 0.5 "VTBlend_Linear" 0.0 false)
      (Input|EnableInput (Variables|Default|GetCharacterRef) (Game|GetPlayerController 0)))))

(event EventBeginPlay
  (bind _asbp_psmoving_wall (Utilities|Casting|CastTobpPSMovingWall (Variables|/Script/Engine.ChildActorComponent|GetChildActor (Variables|Default|GetMovingWall))))
  (Variables|Default|SetMovingWallActor _asbp_psmoving_wall)
  (bind _asbp_character_bp (Utilities|Casting|CastToBP_Character_BP (Game|Player|GetPlayerPawn 0)))
  (Variables|Default|SetCharacterRef _asbp_character_bp))

(event Collision|EventActorBeginOverlap
  (params (OtherActor :type Actor%20Object%20Reference)))

(event EventTick
  (params (DeltaSeconds :type Float%20%28single-precision%29))
  (bind _returnvalue (Game|GetPlayerController 0))
  (if (Variables|Default|GetPuzzleFinished)
    (Utilities|FlowControl|DoOnce false
      (:Completed
        (Utilities|FlowControl|Delay 1.0)
        (Transformation|SetActorLocationAndRotation (Variables|Default|GetFreeLevelCamera) (Transformation|GetWorldLocation (Variables|Default|GetCameraLocation)) (Math|Rotator|FindLookatRotation (Transformation|GetWorldLocation (Variables|Default|GetCameraLocation)) (Transformation|GetWorldLocation (Variables|Default|GetCameraLookat))))
        (Game|Player|SetViewTargetwithBlend (Game|GetPlayerController 0) (Variables|Default|GetFreeLevelCamera) 1.0 "VTBlend_Linear" 0.0 false)
        (Utilities|FlowControl|Delay 1.5)
        (if (Variables|Default|GetPuzzleFinished)
          _
          (else
            (Variables|/Script/WorldSwitching.PSMovingWall|SetActivateMoving (Variables|Default|GetMovingWallActor) true)))
        (Utilities|FlowControl|Delay 2.0)
        (Game|Player|SetViewTargetwithBlend _returnvalue (Pawn|GetControlledPawn _returnvalue) 0.5 "VTBlend_Linear" 0.0 false)
        (Input|EnableInput (Variables|Default|GetCharacterRef) (Game|GetPlayerController 0))))))

(fn ConstructionScript)