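; Puzzle elevator that starts shuttling between ground and a top platform once both child-actor torches are lit and the player steps on it.
; Tick checks the torches, fading in a point light via timeline when both are lit.
; The trigger then freezes player input in an idle pose.
; After a delay, a timeline plays or reverses based on elevator position, restoring input and re-arming the trigger when finished.
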(event OnComponentBeginOverlap(ElevatorTrigger)
  (params (OverlappedComponent :type Primitive%20Component%20Object%20Reference) (OtherActor :type Actor%20Object%20Reference) (OtherComp :type Primitive%20Component%20Object%20Reference) (OtherBodyIndex :type Integer) (bFromSweep :type Boolean) (SweepResult :type Hit%20Result%20Structure%20%28by%20ref%29))
  (bind _returnvalue (Game|GetPlayerCharacter 0))
  ;[1 1 1] The collision freezes the players input and also forces her to a idle animation. I had some issues setting the speed in the blend space here, so I chose to do it this way.
  (if (Variables|Default|GetTorchesLit)
    (if (Variables|Default|GetElevatorSteppedOn)
      _
      (else
        (Variables|Default|SetElevatorSteppedOn true)))
    (bind _asbp_character (Utilities|Casting|CastToBP_Character _returnvalue))
    (Variables|/Script/WorldSwitching.BP_Character|SetRunningAnimations _asbp_character "IDLE")
    (Input|DisableInput _returnvalue 0)
    (Collision|SetCollisionEnabled (Variables|Default|GetElevatorTrigger) "NoCollision")))

(event Custom|MoveElevator
  (bind _elevatorgroundlocation (Variables|Default|GetElevatorGroundLocation))
  (Variables|Default|SetElevatorRunning true) ; This makes sure that the function won't run again while the elevator is moving
  (if (Math|Vector|Equal(Vector) (Transformation|GetWorldLocation (Variables|Default|Getelevator)) (Variables|Default|GetElevatorGroundLocation) 1e+01) ; This makes sure that the elevator goes the right way.\nUp if the location is equal ElevatorGroudnLocation\nDown if it isn't
    (bind _newtrack_0 (Timeline|SmoothlyMovingElevator Play)
      (:Update
        (Transformation|SetWorldLocation (Variables|Default|Getelevator) (Math|Vector|MakeVector (.x _elevatorgroundlocation) (.y _elevatorgroundlocation) (Math|Float|Lerp (.z _elevatorgroundlocation) (.z (Variables|Default|GetTopPlatformLocation)) _newtrack_0)) false false)
        (Collision|SetCollisionEnabled (Variables|Default|GetElevatorTrigger) "NoCollision"))
      (:Finished
        ;[1 1 1] Here I make sure that the collision that  freeze the player works after the player has used the elevator once. I give the player 2 seconds to get off the elevator, or it will go down again
        (Input|EnableInput (Game|GetPlayerCharacter 0) 0)
        (Utilities|FlowControl|Delay 2.0)
        (Collision|SetCollisionEnabled (Variables|Default|GetElevatorTrigger) "QueryOnly")
        (Variables|Default|SetElevatorRunning false)))
    (else
      (Timeline|SmoothlyMovingElevator Reverse))))

(event EventBeginPlay
  ;[1 1 1] Sets up the necessary variables to run the elevator puzzle. This makes it possible to use it in multiple locations, since the variables are set based on the components in each instance of the class
  (bind _asbp_dynamic_torch (Utilities|Casting|CastToBP_DynamicTorch (Variables|/Script/Engine.ChildActorComponent|GetChildActor (Variables|Default|Gettorch1))))
  (Variables|Default|SetTorch1Ref _asbp_dynamic_torch)
  (bind _asbp_dynamic_torch_2 (Utilities|Casting|CastToBP_DynamicTorch (Variables|/Script/Engine.ChildActorComponent|GetChildActor (Variables|Default|Gettorch2))))
  (Variables|Default|SetTorch2Ref _asbp_dynamic_torch_2)
  (Variables|Default|SetElevatorGroundLocation (Transformation|GetWorldLocation (Variables|Default|Getelevator)))
  (Variables|Default|SetTopPlatformLocation (Transformation|GetWorldLocation (Variables|Default|Gettop%20plattform))))

(event Collision|EventActorBeginOverlap
  (params (OtherActor :type Actor%20Object%20Reference)))

(event EventTick
  (params (DeltaSeconds :type Float%20%28single-precision%29))
  (if (and (Variables|Default|GetElevatorSteppedOn) (not (Variables|Default|GetElevatorRunning)))
    ;[1 1 1] moves the elevator with a 2 seconds delay in between, after the player have stepped on it once and lit the torches
    (Utilities|FlowControl|Delay 2.0)
    (CallFunction|MoveElevator)
    (else
      ;[1 1 1] This section deals with lighting torches. If the torches are lit, the boolean TorchesLit is set, which is one demand for the elevator to start running. It also ticks off a light that starts lighting up the elevator
      (if (and (Variables|/Game/Blueprints/WorldActors/Both/BP_DynamicTorch.BP_DynamicTorch_C|GetbIsLit (Variables|Default|GetTorch1Ref)) (Variables|/Game/Blueprints/WorldActors/Both/BP_DynamicTorch.BP_DynamicTorch_C|GetbIsLit (Variables|Default|GetTorch2Ref)))
        (Utilities|FlowControl|DoOnce false
          (:Completed
            (Variables|Default|SetTorchesLit true)
            (bind _newtrack_0 (Timeline|LightTimeline PlayFromStart)
              (:Update
                (Rendering|Components|Light|SetIntensity (Variables|Default|GetPointLight) _newtrack_0)))))))))

(fn ConstructionScript)