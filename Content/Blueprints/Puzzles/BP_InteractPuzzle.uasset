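; Puzzle actor that opens a moving wall and activates a portal once both of its torches are lit.
; BeginPlay caches the torch and wall child actors plus the player character.
; Tick polls both lit states, then a DoOnce runs a delayed cutscene: the view blends to a repositioned free camera aimed at a look-at point, the wall moves, the portal activates, and the view returns to the pawn.
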(event EventBeginPlay
  (bind _asbp_dynamic_torch (Utilities|Casting|CastToBP_DynamicTorch (Variables|/Script/Engine.ChildActorComponent|GetChildActor (Variables|Default|Gettorch1))))
  (Variables|Default|SetTorchActor1 _asbp_dynamic_torch)
  (bind _asbp_dynamic_torch_2 (Utilities|Casting|CastToBP_DynamicTorch (Variables|/Script/Engine.ChildActorComponent|GetChildActor (Variables|Default|Gettorch2))))
  (Variables|Default|SetTorchActor2 _asbp_dynamic_torch_2)
  (bind _asbp_psmoving_wall (Utilities|Casting|CastTobpPSMovingWall (Variables|/Script/Engine.ChildActorComponent|GetChildActor (Variables|Default|GetMovingWall))))
  (Variables|Default|SetMovingWallActor _asbp_psmoving_wall)
  (bind _asbp_character_bp (Utilities|Casting|CastToBP_Character_BP (Game|Player|GetPlayerPawn 0)))
  (Variables|Default|SetCharacterRef _asbp_character_bp))

(event Collision|EventActorBeginOverlap
  (params (OtherActor :type Actor%20Object%20Reference)))

(event EventTick
  (params (DeltaSeconds :type Float%20%28single-precision%29))
  (bind _returnvalue (Game|GetPlayerController 0))
  (if (and (Variables|/Game/Blueprints/WorldActors/Both/BP_DynamicTorch.BP_DynamicTorch_C|GetbIsLit (Variables|Default|GetTorchActor1)) (Variables|/Game/Blueprints/WorldActors/Both/BP_DynamicTorch.BP_DynamicTorch_C|GetbIsLit (Variables|Default|GetTorchActor2)))
    (Utilities|FlowControl|DoOnce false
      (:Completed
        (Utilities|FlowControl|Delay 1.0)
        (Transformation|SetActorLocationAndRotation (Variables|Default|GetFreeLevelCamera) (Transformation|GetWorldLocation (Variables|Default|GetCameraLocation)) (Math|Rotator|FindLookatRotation (Transformation|GetWorldLocation (Variables|Default|GetCameraLocation)) (Transformation|GetWorldLocation (Variables|Default|GetCameraLookat))))
        (Game|Player|SetViewTargetwithBlend (Game|GetPlayerController 0) (Variables|Default|GetFreeLevelCamera) 1.0 "VTBlend_Linear" 0.0 false)
        (Utilities|FlowControl|Delay 1.5)
        (Variables|/Script/WorldSwitching.PSMovingWall|SetActivateMoving (Variables|Default|GetMovingWallActor) true)
        (Utilities|FlowControl|Delay 2.0)
        (Class|PSPortal|Activate (Variables|Default|GetPortal) false)
        (Utilities|FlowControl|Delay 1.5)
        (Game|Player|SetViewTargetwithBlend _returnvalue (Pawn|GetControlledPawn _returnvalue) 0.5 "VTBlend_Linear" 0.0 false)))))

(fn ConstructionScript)