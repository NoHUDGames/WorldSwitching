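; Tutorial world-change puzzle actor that drives a rotating bladed cross and two skull artifacts that reverse its spin.
; A one-shot box trigger shakes the camera, emits particles briefly and ramps up a timeline-driven rotation speed that Tick applies to the cross.
; Overlapping either artifact's sphere shakes the camera and plays the reversal timeline forward or backward based on current speed.
; A second one-shot box animates both artifacts' light intensity.
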(event OnComponentBeginOverlap(BoxCollider)
  (params (OverlappedComponent :type Primitive%20Component%20Object%20Reference) (OtherActor :type Actor%20Object%20Reference) (OtherComp :type Primitive%20Component%20Object%20Reference) (OtherBodyIndex :type Integer) (bFromSweep :type Boolean) (SweepResult :type Hit%20Result%20Structure%20%28by%20ref%29))
  (Collision|SetCollisionEnabled (Variables|Default|GetBoxCollider) "NoCollision")
  (Actor|Tick|SetActorTickEnabled true)
  (CallFunction|ActivationSequence true)
  (Utilities|FlowControl|Delay 3.0)
  (Components|Activation|Deactivate (Variables|Default|GetParticleSystem))
  (bind _rotateblades (Timeline|Timeline_0 PlayFromStart)
    (:Update
      (Variables|Default|SetRotateSpeedAmount _rotateblades))))

(event OnComponentBeginOverlap(Box)
  (params (OverlappedComponent :type Primitive%20Component%20Object%20Reference) (OtherActor :type Actor%20Object%20Reference) (OtherComp :type Primitive%20Component%20Object%20Reference) (OtherBodyIndex :type Integer) (bFromSweep :type Boolean) (SweepResult :type Hit%20Result%20Structure%20%28by%20ref%29))
  (Collision|SetCollisionEnabled OverlappedComponent "NoCollision")
  (bind _asskull_artifact (Utilities|Casting|CastToSkullArtifact (Variables|/Script/Engine.ChildActorComponent|GetChildActor (Variables|Default|GetArtifact2))))
  (bind _asskull_artifact_2 (Utilities|Casting|CastToSkullArtifact (Variables|/Script/Engine.ChildActorComponent|GetChildActor (Variables|Default|GetArtifact))))
  (bind _newtrack_0 (Timeline|FadeUpDownLight PlayFromStart)
    (:Update
      (Rendering|Components|Light|SetIntensity (Variables|/Game/Blueprints/WorldActors/Physical/SkullArtifact.SkullArtifact_C|GetPointLight _asskull_artifact_2) _newtrack_0)
      (Rendering|Components|Light|SetIntensity (Variables|/Game/Blueprints/WorldActors/Physical/SkullArtifact.SkullArtifact_C|GetPointLight _asskull_artifact) _newtrack_0))))

(event Custom|TriggerReverse1
  (params (OverlappedComponent :type Primitive%20Component%20Object%20Reference) (OtherActor :type Actor%20Object%20Reference) (OtherComp :type Primitive%20Component%20Object%20Reference) (OtherBodyIndex :type Integer) (bFromSweep :type Boolean) (SweepResult :type Hit%20Result%20Structure%20%28by%20ref%29))
  (Development|PrintText "TriggeredEvent")
  (CallFunction|ReverseRotation))

(event Custom|TriggerReverse2
  (params (OverlappedComponent :type Primitive%20Component%20Object%20Reference) (OtherActor :type Actor%20Object%20Reference) (OtherComp :type Primitive%20Component%20Object%20Reference) (OtherBodyIndex :type Integer) (bFromSweep :type Boolean) (SweepResult :type Hit%20Result%20Structure%20%28by%20ref%29))
  (Development|PrintText "TriggeredEvent")
  (CallFunction|ReverseRotation))

(event Custom|ReverseRotation
  (CallFunction|ActivationSequence false)
  (Math|Float|CompareFloat (Variables|Default|GetRotateSpeedAmount) 1.0
    (:>
      (bind _newtrack_0 (Timeline|ReverseToClockwise PlayFromStart)
        (:Update
          (Variables|Default|SetRotateSpeedAmount _newtrack_0))
        (:Finished
          (Components|Activation|Deactivate (Variables|Default|GetParticleSystem)))))
    (:<
      (Timeline|ReverseToClockwise ReverseFromEnd))))

(event EventBeginPlay
  (bind _asbp_character (Utilities|Casting|CastToBP_Character (Game|Player|GetPlayerPawn 0)))
  (Variables|Default|SetPawnRef _asbp_character)
  (bind _asskull_artifact (Utilities|Casting|CastToSkullArtifact (Variables|/Script/Engine.ChildActorComponent|GetChildActor (Variables|Default|GetArtifact)))
    (:then
      (Collision|AssignOnComponentBeginOverlap (Actor|GetComponentbyClass _asskull_artifact "/Script/Engine.SphereComponent") (delegate Custom|TriggerReverse1))
      (bind _asskull_artifact_2 (Utilities|Casting|CastToSkullArtifact (Variables|/Script/Engine.ChildActorComponent|GetChildActor (Variables|Default|GetArtifact2))))
      (Collision|AssignOnComponentBeginOverlap (Actor|GetComponentbyClass _asskull_artifact_2 "/Script/Engine.SphereComponent") (delegate Custom|TriggerReverse2)))
    (:CastFailed
      (Development|PrintText "CastFailed"))))

(event Collision|EventActorBeginOverlap
  (params (OtherActor :type Actor%20Object%20Reference)))

(event EventTick
  (params (DeltaSeconds :type Float%20%28single-precision%29))
  (Transformation|AddRelativeRotation (Variables|Default|GetCross1) (Math|Rotator|MakeRotator 0.0 0.0 (* DeltaSeconds (Variables|Default|GetRotateSpeedAmount))) false false))

(fn ConstructionScript)

(fn ActivationSequence
  (params (smoke :type Boolean))
  (Camera|PlayWorldCameraShake "/Game/Blueprints/CameraShakes/SpiralPopUpShake.SpiralPopUpShake_C" (Transformation|GetActorLocation (Game|Player|GetPlayerPawn 0)) 1e+03 2e+03)
  (if smoke
    (Components|Activation|Activate (Variables|Default|GetParticleSystem) false)))