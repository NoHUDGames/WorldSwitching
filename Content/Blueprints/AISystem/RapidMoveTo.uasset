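; Behavior tree task that moves a Spirit or Shaman enemy toward the blackboard's TargetToFollow actor with its movement animation set.
; It caches controller and pawn references, branching on the owning controller's class, then runs AI MoveTo and finishes successfully when the move finishes.
; If CanChase is set, a looping one-second timer counts down five seconds, printing each tick, then sets CanChase false and empties TargetToFollow.
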(event EventReceiveExecute
  (params (OwnerActor :type Actor%20Object%20Reference))
  (CallFunction|SettingUpVariables OwnerActor)
  (if (== (Utilities|GetClass OwnerActor) 0)
    (Variables|/Script/WorldSwitching.SpiritTest|SetRunningAnimations (Variables|Default|GetSpiritEnemyRef) "MOVEMENT")
    (AI|AIMoveTo (Variables|Default|GetSpiritEnemyControllerRef) "0, 0, 0" (AI|BehaviorTree|GetBlackboardValueasActor (Variables|Default|GetTargetToFollow)) -1.0 "Default" "Default" true true
      (:then
        (if (Class|BTFunctionLibrary|GetBlackboardValueasBool (Variables|Default|GetCanChase)) :!label _label
          (Variables|Default|SetChasingTimer 5)
          (Utilities|Time|SetTimerbyFunctionName 0 "ChasingCountdown" 1.0 true)))
      (:OnMoveFinished
        (AI|BehaviorTree|FinishExecute true :!label _label_2)))
    (else
      (Variables|/Script/WorldSwitching.PShamanEnemy|SetRunningAnimations (Variables|Default|GetShamanEnemyRef) "MOVEMENT")
      (AI|AIMoveTo (Variables|Default|GetShamanEnemyControllerRef) "0, 0, 0" (AI|BehaviorTree|GetBlackboardValueasActor (Variables|Default|GetTargetToFollow)) -1.0 "Default" "Default" true true
        (:then
          (goto _label))
        (:OnMoveFinished
          (goto _label_2))))))

(fn ChasingCountdown
  (if (> (Variables|Default|GetChasingTimer) 0)
    (bind _result (Math|Integer|DecrementInt (Variables|Default|GetChasingTimer))
      (:%20%20
        (bind _output_get (Variables|Default|SetChasingTimer _result))
        (Development|PrintString (Utilities|String|ToString(Integer) _output_get))))
    (else
      (Class|BTFunctionLibrary|SetBlackboardValueasBool (Variables|Default|GetCanChase) false)
      (Class|BTFunctionLibrary|SetBlackboardValueasObject (Variables|Default|GetTargetToFollow)))))

(fn SettingUpVariables
  (params (OwnerActor :type Actor%20Object%20Reference))
  (if (!= (Variables|Default|GetBP_CharacterRef) 0)
    _
    (else
      (bind _asbp_character (Utilities|Casting|CastToBP_Character (Pawn|GetControlledPawn (Game|GetPlayerController 0))))
      (Variables|Default|SetBP_CharacterRef _asbp_character)))
  (if (== (Utilities|GetClass OwnerActor) "/Game/Blueprints/AISystem/SpiritEnemyAI/SpiritEnemyController.SpiritEnemyController_C")
    (if (== (Variables|Default|GetSpiritEnemyControllerRef) 0)
      (bind _asspirit_enemy_controller (Utilities|Casting|CastToSpiritEnemyController OwnerActor))
      (bind _output_get (Variables|Default|SetSpiritEnemyControllerRef _asspirit_enemy_controller)))
    (if (== (Variables|Default|GetSpiritEnemyRef) 0)
      (bind _asbp_spirit_test (Utilities|Casting|CastToBP_SpiritTest (Pawn|GetControlledPawn _output_get)))
      (Variables|Default|SetSpiritEnemyRef _asbp_spirit_test))
    (else
      (if (== (Variables|Default|GetShamanEnemyControllerRef) 0)
        (bind _asshaman_enemy_controller (Utilities|Casting|CastToShamanEnemyController OwnerActor))
        (bind _output_get_2 (Variables|Default|SetShamanEnemyControllerRef _asshaman_enemy_controller)))
      (if (== (Variables|Default|GetShamanEnemyRef) 0)
        (bind _asbp_pshaman_enemy (Utilities|Casting|CastToBP_PShamanEnemy (Pawn|GetControlledPawn _output_get_2)))
        (Variables|Default|SetShamanEnemyRef _asbp_pshaman_enemy)))))