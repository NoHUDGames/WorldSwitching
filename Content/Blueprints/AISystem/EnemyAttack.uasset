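; Behavior tree task in which an enemy run by SpiritEnemyController attacks the player's BP_Character.
; On execute it caches the owning controller and the player's pawn, prints a debug message, waits briefly, then decrements the character's Lives and finishes successfully.
; It makes no range or hit check, and a failed cast leaves the task without a FinishExecute call.
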(event EventReceiveExecute
  (params (OwnerActor :type Actor%20Object%20Reference))
  (if (!= (Variables|Default|GetSpiritEnemyControllerRef) 0)
    _
    (else
      (bind _asspirit_enemy_controller (Utilities|Casting|CastToSpiritEnemyController OwnerActor))
      (Variables|Default|SetSpiritEnemyControllerRef _asspirit_enemy_controller)))
  (if (!= (Variables|Default|GetBP_CharacterRef) 0)
    _
    (else
      (bind _asbp_character (Utilities|Casting|CastToBP_Character (Pawn|GetControlledPawn (Game|GetPlayerController 0))))
      (Variables|Default|SetBP_CharacterRef _asbp_character)))
  (Development|PrintString "Attacking Enemy")
  (Utilities|FlowControl|Delay 1.0)
  (Math|Integer|DecrementInt (Variables|/Script/WorldSwitching.BP_Character|GetLives (Variables|Default|GetBP_CharacterRef))
    (:%20%20
      (AI|BehaviorTree|FinishExecute true))))