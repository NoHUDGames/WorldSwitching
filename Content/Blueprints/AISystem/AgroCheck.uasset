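; Behavior tree service that lets spirit enemies notice and target the player.
; Each tick it sphere-traces around the controlled pawn within NoticePlayerRadius, ignoring other spirits, then line-traces on the Camera channel to each hit to confirm line of sight.
; A visible hit while the player has lives sets the TargetToFollow and TargetLocation blackboard keys; a failed check clears TargetToFollow.
; Controller and player character references are cached on first use.
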(event EventTick
  (params (OwnerActor :type Actor%20Object%20Reference) (DeltaSeconds :type Float%20%28single-precision%29))
  (if (!= (Variables|Default|GetSpiritEnemyControllerRef) 0)
    _
    (else
      (bind _asspirit_enemy_controller (Utilities|Casting|CastToSpiritEnemyController OwnerActor))
      (Variables|Default|SetSpiritEnemyControllerRef _asspirit_enemy_controller)))
  (if (!= (Variables|Default|GetBP_CharacterRef) 0)
    _
    (else
      (bind _asbp_character (Utilities|Casting|CastToBP_Character (Pawn|GetControlledPawn (Game|GetPlayerController 0))))
      (Variables|Default|SetBP_CharacterRef _asbp_character)))
  (bind _outactors (Actor|GetAllActorsOfClass "/Game/Blueprints/BP_SpiritTest.BP_SpiritTest_C"))
  (Variables|Default|SetMyLocation (Transformation|GetActorLocation (Pawn|GetControlledPawn (Variables|Default|GetSpiritEnemyControllerRef))))
  (bind _outhits (Collision|MultiSphereTraceForObjects (Transformation|GetActorLocation (Pawn|GetControlledPawn (Variables|Default|GetSpiritEnemyControllerRef))) (+ (Transformation|GetActorLocation (Pawn|GetControlledPawn (Variables|Default|GetSpiritEnemyControllerRef))) "0, 0,15.000000") (Variables|Default|GetNoticePlayerRadius) (Variables|Default|GetDesiredObjectTypes) false _outactors "None"))
  (bind _array_element (Utilities|Array|ForEachLoopwithBreak _outhits)
    (:LoopBody
      (bind _outhit (Collision|LineTraceByChannel (Variables|Default|GetMyLocation) (Transformation|GetActorLocation (.HitActor (Collision|BreakHitResult _array_element))) "TraceTypeQuery2" false _outactors "None"))
      (if (and (== (.HitActor (Collision|BreakHitResult _outhit)) (.HitActor (Collision|BreakHitResult _array_element))) (> (Variables|/Script/WorldSwitching.BP_Character|GetLives (Variables|Default|GetBP_CharacterRef)) 0))
        (Class|BTFunctionLibrary|SetBlackboardValueasObject (Variables|Default|GetTargetToFollow) (.HitActor (Collision|BreakHitResult _outhit)))
        (AI|BehaviorTree|SetBlackboardValueasVector (Variables|Default|GetTargetLocation) (Transformation|GetActorLocation (.HitActor (Collision|BreakHitResult _outhit))))
        (else
          (Class|BTFunctionLibrary|SetBlackboardValueasObject (Variables|Default|GetTargetToFollow)))))))