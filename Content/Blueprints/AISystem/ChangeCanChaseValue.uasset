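; Behavior tree task for the spirit enemy that re-enables chasing and clears its current follow target.
; On execute, it lazily casts and caches the SpiritEnemyController from the owner and the BP_SpiritTest pawn it controls.
; It then sets the pawn's animation state to idle, sets CanChase to true, empties TargetToFollow on the blackboard and finishes successfully.
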(event EventReceiveExecute
  (params (OwnerActor :type Actor%20Object%20Reference))
  (if (!= (Variables|Default|GetSpiritEnemyControllerRef) 0)
    _
    (else
      (bind _asspirit_enemy_controller (Utilities|Casting|CastToSpiritEnemyController OwnerActor))
      (bind _output_get (Variables|Default|SetSpiritEnemyControllerRef _asspirit_enemy_controller))))
  (if (!= (Variables|Default|GetBP_SpiritEnemyRef) 0)
    _
    (else
      (bind _asbp_spirit_test (Utilities|Casting|CastToBP_SpiritTest (Pawn|GetControlledPawn _output_get)))
      (bind _output_get_2 (Variables|Default|SetBP_SpiritEnemyRef _asbp_spirit_test))))
  (Variables|/Script/WorldSwitching.SpiritTest|SetRunningAnimations _output_get_2 "IDLE")
  (Class|BTFunctionLibrary|SetBlackboardValueasBool (Variables|Default|GetCanChase) true)
  (Class|BTFunctionLibrary|SetBlackboardValueasObject (Variables|Default|GetTargetToFollow))
  (AI|BehaviorTree|FinishExecute true))