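; Behavior tree decorator that checks how far a spirit enemy's pawn is from its follow target.
; It casts the owner to SpiritEnemyController, stores that reference, and measures the distance from the controlled pawn to the TargetToFollow blackboard actor.
; Despite the CloseEnough name, it passes when that distance is at or beyond AcceptableDistance.
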(fn PerformConditionCheck
  (params (OwnerActor :type Actor%20Object%20Reference))
  (bind _asspirit_enemy_controller (Utilities|Casting|CastToSpiritEnemyController OwnerActor))
  (Variables|Default|SetSpiritEnemyControllerRef _asspirit_enemy_controller)
  (return (>= (Math|Vector|VectorLength (- (Transformation|GetActorLocation (AI|BehaviorTree|GetBlackboardValueasActor (Variables|Default|GetTargetToFollow))) (Transformation|GetActorLocation (Pawn|GetControlledPawn (Variables|Default|GetSpiritEnemyControllerRef))))) (Variables|Default|GetAcceptableDistance))))